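; BP_FadeActor is a mesh actor that fades out and back in through a "Fade" material parameter.
; Construction caches the original materials and creates dynamic instances from fade materials, which FadeOut swaps onto the mesh.
; FadeOut plays a timeline driving the parameter, and Fadein reverses it.
; On finish, a value of one restores original materials; BlockVisbilites optionally makes Visibility collision block at one and ignore at zero.
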(event EventBeginPlay)

(event Collision|EventActorBeginOverlap
  (params (OtherActor :type Actor%20Object%20Reference)))

(event EventTick
  (params (DeltaSeconds :type Float%20%28single-precision%29)))

(event EventFadeOut
  (CallFunction|SetMaterialtoDynamicsInstances)
  (bind _fade (Timeline|FadeTimeLine Play)
    (:Update
      (for _array_element (Variables|Default|GetDynamicMaterialInst)
        (Rendering|Material|SetScalarParameterValue _array_element "Fade" _fade :!class /Script/Engine.MaterialInstanceDynamic)))
    (:Finished
      (CallFunction|FadeFinished _fade))))

(event EventFadein
  (bind _fade (Timeline|FadeTimeLine Reverse)
    (:Update
      (for _array_element (Variables|Default|GetDynamicMaterialInst)
        (Rendering|Material|SetScalarParameterValue _array_element "Fade" _fade :!class /Script/Engine.MaterialInstanceDynamic)))
    (:Finished
      (CallFunction|FadeFinished _fade))))

(fn ConstructionScript
  (Utilities|Array|Clear (Variables|Default|GetDynamicMaterialInst))
  (Variables|Default|SetOrginalMaterials (Rendering|Material|GetMaterials (Variables|Default|GetMesh)))
  (for _array_element (Variables|Default|GetFadeMaterialInstance)
    (bind _returnvalue (Rendering|Material|CreateDynamicMaterialInstance _array_element "None" "None" :!class /Script/Engine.KismetMaterialLibrary))
    (Utilities|Array|AddUnique (Variables|Default|GetDynamicMaterialInst) _returnvalue)))

(fn SetMaterialtoDynamicsInstances
  (for (_array_element _array_index) (Variables|Default|GetDynamicMaterialInst)
    (Rendering|Material|SetMaterial (Variables|Default|GetMesh) _array_index _array_element)))

(fn ResetMaterials
  (for (_array_element _array_index) (Variables|Default|GetOrginalMaterials)
    (Rendering|Material|SetMaterial (Variables|Default|GetMesh) _array_index _array_element)))

(fn FadeFinished
  (params (InputPin :type Float%20%28single-precision%29))
  (if (>= InputPin 1.0)
    (CallFunction|ResetMaterials)
    (if (Variables|Default|GetBlockVisbilites)
      (Collision|SetCollisionResponsetoChannel (Variables|Default|GetMesh) "ECC_Visibility" "ECR_Block"))
    (elif (<= InputPin 0.0)
      (if (Variables|Default|GetBlockVisbilites)
        (Collision|SetCollisionResponsetoChannel (Variables|Default|GetMesh) "ECC_Visibility" "ECR_Ignore")))))