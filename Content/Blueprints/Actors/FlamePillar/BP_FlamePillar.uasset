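; BP_FlamePillar is a flame pillar actor that gives its fire light a randomly varying flicker.
; On BeginPlay it randomly picks one of two timelines, and each picks again when it finishes, forming an endless loop.
; Each timeline's intensity curve drives ScaleFlameIntensity, which sets the FireLight intensity as a multiple of BaseIntensity.
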(event Custom|StartTimeline_1
  (bind _flameintensity (Timeline|FlameIntensity_1 Play)
    (:Update
      (CallFunction|ScaleFlameIntensity _flameintensity))
    (:Finished
      (CallFunction|ChoseTimeLine))))

(event Custom|StartTimeLine_2
  (bind _flameintensity (Timeline|FlameInvensity_2 Play)
    (:Update
      (CallFunction|ScaleFlameIntensity _flameintensity))
    (:Finished
      (CallFunction|ChoseTimeLine))))

(event Custom|ChoseTimeLine
  (switch int (Math|Random|RandomIntegerinRange 0 1)
    (:Default
      (CallFunction|StartTimeLine2 :!label _label))
    (:0
      (CallFunction|StartTimeline1))
    (:1
      (goto _label))))

(event EventBeginPlay
  (CallFunction|ChoseTimeLine))

(event Collision|EventActorBeginOverlap
  (params (OtherActor :type Actor%20Object%20Reference)))

(event EventTick
  (params (DeltaSeconds :type Float%20%28single-precision%29)))

(fn ConstructionScript)

(fn ScaleFlameIntensity
  (params (Intensity :type Float%20%28double-precision%29))
  (Rendering|Components|Light|SetIntensity (Variables|Default|GetFireLight) (* Intensity (Variables|Default|GetBaseIntensity))))